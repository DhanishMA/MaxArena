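; HeroController_BP is a hero controller Blueprint that lets the player cycle between characters with two number keys.
; Key 1 steps forward and key 2 steps back by passing the adjusted Index to SwitchCharacter, whose body is not defined in these graphs.
; The returned value becomes the new Index and is printed to screen, and the construction script is empty.
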(event `Key|One`
  (params (Key :type "Key Structure"))
  (:`Pressed`
    (bind _returnvalue (`self.SwitchCharacter` (+ (`self.Index`) 1)))
    (bind _output_get (set `self.Index` _returnvalue))
    (`KismetSystemLibrary.PrintString` (`KismetStringLibrary.Conv_IntToString` _output_get))))

(event `Key|Two`
  (params (Key :type "Key Structure"))
  (:`Pressed`
    (bind _returnvalue (`self.SwitchCharacter` (- (`self.Index`) 1)))
    (bind _output_get (set `self.Index` _returnvalue))
    (`KismetSystemLibrary.PrintString` (`KismetStringLibrary.Conv_IntToString` _output_get))))

(fn `UserConstructionScript`)